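; ExitHatch is a level exit actor that advances the game to the next numbered level when its Box is overlapped.
; On overlap, with no check on what entered, it parses the number after the "Level" prefix of the current level name, increments it and rebuilds the name.
; It prints that name, then opens it, or opens MainMenu instead when the result is the hard-coded Level4.
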(event `self.Box.OnComponentBeginOverlap`
  (params (OverlappedComponent :type "PrimitiveComponent Object Reference") (OtherActor :type "Actor Object Reference") (OtherComp :type "PrimitiveComponent Object Reference") (OtherBodyIndex :type Integer) (bFromSweep :type Boolean) (SweepResult :type "HitResult Structure (by ref)"))
  (bind _returnvalue (`GameplayStatics.GetCurrentLevelName` true))
  (bind _returnvalue_2 (`KismetStringLibrary.Concat_StrStr` "Level" (`KismetStringLibrary.Conv_IntToString` (+ (`KismetStringLibrary.Conv_StringToInt` (`KismetStringLibrary.RightChop` _returnvalue 5)) 1))))
  (`KismetSystemLibrary.PrintString` _returnvalue_2)
  (bind _returnvalue_3 (`KismetStringLibrary.Conv_StringToName` _returnvalue_2))
  (if (== _returnvalue_3 "Level4")
    (`GameplayStatics.OpenLevel` "MainMenu")
    (else
      (`GameplayStatics.OpenLevel` _returnvalue_3))))

(fn `UserConstructionScript`)