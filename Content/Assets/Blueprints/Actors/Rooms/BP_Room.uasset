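; BP_Room is a room actor that spawns a small batch of Enemy actors on its floor through a SpawnEnemies event.
; Spawn points come from the Floor component's bounds, randomized within an inset along X and placed just above the surface.
; The Y spread is scaled to zero, so enemies line up on the floor's center line, with collision handling adjusting positions but always spawning.
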(event `SpawnEnemies`
  (bind (_origin _boxextent) (`KismetSystemLibrary.GetComponentBounds` (`self.Floor`)))
  (bind _returnvalue (* (.x _boxextent) 0.8))
  (bind _returnvalue_2 (* (.y _boxextent) 0.0))
  (for _ (range 3)
    (`|SpawnActorFromClass` "/Game/Assets/Blueprints/Characters/Enemy/Enemy.Enemy_C" (`KismetMathLibrary.Conv_VectorToTransform` (`KismetMathLibrary.MakeVector` (+ (`KismetMathLibrary.RandomFloatInRange` (* _returnvalue -1.0) _returnvalue) (.x _origin)) (+ (`KismetMathLibrary.RandomFloatInRange` (* _returnvalue_2 -1.0) _returnvalue_2) (.y _origin)) (+ (.z _origin) (.z _boxextent) 10.0))) "AdjustIfPossibleButAlwaysSpawn" "OverrideRootScale" null null)))

(fn `UserConstructionScript`)