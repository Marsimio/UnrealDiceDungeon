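; Inventory component that holds ten item slots and displays them in a WB_Inventory widget.
; IA_Inventory toggles the widget along with the cursor and input mode.
; IA_Pickup sphere-traces near the player's feet for a BP_Item, stores it in an empty slot, refreshes the widget and destroys the actor.
; Its stacking branch requires a combined quantity of zero or less, so positive quantities never stack.
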(event `self.ReceiveBeginPlay`
  (bind _returnvalue (`|CreateWidget` "/Game/UI/Inventory/WB_Inventory.WB_Inventory_C"))
  (set `self.InventoryWidget` _returnvalue)
  (`KismetArrayLibrary.Array_Resize` (`self.Items`) 10)
  (`/Game/UI/Inventory/WB_Inventory.LoadInventory` (`self.InventoryWidget`) self))

(event `EnhancedInput|/Game/Inputs/IA_Inventory`
  (params (ActionValue :type Boolean) (ElapsedSeconds :type "Float (double-precision)") (TriggeredSeconds :type "Float (double-precision)") (InputAction :type "InputAction Object Reference" :default "/Game/Inputs/IA_Inventory.IA_Inventory"))
  (bind _returnvalue (`GameplayStatics.GetPlayerController` 0))
  (bind _returnvalue_2 (`GameplayStatics.GetPlayerController` 0))
  (bind _inventorywidget (`self.InventoryWidget`))
  (:`Started`
    (if (`Widget.IsVisible` (`self.InventoryWidget`))
      (`Widget.RemoveFromParent` _inventorywidget)
      (set `PlayerController.bShowMouseCursor` false _returnvalue)
      (`WidgetBlueprintLibrary.SetInputMode_GameOnly` _returnvalue)
      (else
        (set `PlayerController.bShowMouseCursor` true _returnvalue_2)
        (`WidgetBlueprintLibrary.SetInputMode_GameAndUIEx` _returnvalue_2 null)
        (`UserWidget.AddToViewport` _inventorywidget 0)))))

(event `EnhancedInput|/Game/Inputs/IA_Pickup`
  (params (ActionValue :type Boolean) (ElapsedSeconds :type "Float (double-precision)") (TriggeredSeconds :type "Float (double-precision)") (InputAction :type "InputAction Object Reference" :default "/Game/Inputs/IA_Pickup.IA_Pickup"))
  (bind _returnvalue (- (`Actor.K2_GetActorLocation` (`GameplayStatics.GetPlayerCharacter` 0)) (0.0 0.0 65.0)))
  (:`Started`
    (bind _outhit (`KismetSystemLibrary.SphereTraceSingle` :`Start` _returnvalue :`End` _returnvalue :`Radius` 240.0 :`TraceChannel` "TraceTypeQuery1" :`DrawDebugType` "ForDuration"))
    (bind _asbp_item (cast `/Game/Assets/Blueprints/Structure/Items/BP_Item` (`.HitActor` (`GameplayStatics.BreakHitResult` _outhit))))
    (for (_array_element _array_index) (`self.Items`)
      (`/Engine/EditorBlueprintResources/StandardMacros.IsValid` _asbp_item
        (:`Is Valid`
          (bind (_name _stackable _quantity) (break `/Game/Assets/Blueprints/Structure/Items/S_ItemStruct` _array_element))
          (bind (_name_2 _stackable_2 _quantity_2) (break `/Game/Assets/Blueprints/Structure/Items/S_ItemStruct` (`/Game/Assets/Blueprints/Structure/Items/BP_Item.Item` _asbp_item)))
          (bind _returnvalue_2 (+ _quantity _quantity_2))
          (if (and (`KismetTextLibrary.EqualEqual_TextText` _name _name_2) _stackable_2 (<= _returnvalue_2 0))
            (bind (_item_name _item_stackable _item_quantity _item_thumbnail _item_mesh) (break `/Game/Assets/Blueprints/Structure/Items/S_ItemStruct` (`/Game/Assets/Blueprints/Structure/Items/BP_Item.Item` _asbp_item)))
            (`KismetArrayLibrary.Array_Set` (`self.Items`) _array_index (make `/Game/Assets/Blueprints/Structure/Items/S_ItemStruct` _item_name _item_stackable _returnvalue_2 _item_thumbnail _item_mesh))
            (`/Game/UI/Inventory/WB_Inventory.LoadInventory` (`self.InventoryWidget`) self :!label _label)
            (`Actor.K2_DestroyActor` _asbp_item)
            (elif (== _quantity 0)
              (`KismetArrayLibrary.Array_Set` (`self.Items`) _array_index (`/Game/Assets/Blueprints/Structure/Items/BP_Item.Item` _asbp_item))
              (goto _label))))))))